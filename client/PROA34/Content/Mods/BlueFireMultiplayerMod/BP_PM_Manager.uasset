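; Manager actor for the Blue Fire multiplayer mod that represents other players as BP_PM_Ghost actors.
; Tick caches the player character and sets Run when the level is MainMenu; BeginPlay, if Run, passes the player's transform to an empty SyncInfo stub.
; UpdateGhosts, not called here, spawns colored, named ghosts or teleports existing ones through an ID-keyed map, and destroys those listed for removal.
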(event `self.ReceiveBeginPlay`
  (if (`self.Run`)
    (bind _info (`self.MakePlayerInfo`))
    (`self.SyncInfo` _info)))

(event `self.ReceiveTick`
  (params (DeltaSeconds :type "Float (single-precision)"))
  (bind _returnvalue (`GameplayStatics.GetActorOfClass` "/Game/BlueFire/Player/Logic/Player_Character_BP.Player_Character_BP_C"))
  (set `self.PlayerRef` _returnvalue)
  (bind _returnvalue_2 (`GameplayStatics.GetCurrentLevelName` true))
  (set `self.Run` (`KismetStringLibrary.EqualEqual_StrStr` _returnvalue_2 "MainMenu")))

(fn `MakePlayerInfo`
  (returns (Info :type "/Game/Mods/BlueFireMultiplayerMod/ST_PlayerInfo Structure"))
  (bind _returnvalue (`self.GetTransform` (`self.PlayerRef`)))
  (return (make `/Game/Mods/BlueFireMultiplayerMod/ST_PlayerInfo` (.x (.location _returnvalue)) (.y (.location _returnvalue)) (.z (.location _returnvalue)) (.roll (.rotation _returnvalue)) (.pitch (.rotation _returnvalue)) (.yaw (.rotation _returnvalue)))))

(fn `RemoveGhost`
  (params (id :type Byte))
  (bind _ghosts (`self.Ghosts`))
  (`self.K2_DestroyActor` (`BlueprintMapLibrary.Map_Find` _ghosts id))
  (`BlueprintMapLibrary.Map_Remove` _ghosts id))

(fn `SpawnGhost`
  (params (info :type "/Game/Mods/BlueFireMultiplayerMod/ST_PlayerInfo Structure"))
  (`|SpawnActorFromClass` "/Game/Mods/BlueFireMultiplayerMod/BP_PM_Ghost.BP_PM_Ghost_C" (`KismetMathLibrary.MakeTransform` (`KismetMathLibrary.MakeVector` info_location_x_2_DE92424E446ED6A7C5A5868276BA5D20 info_location_y_9_2173608E4FFA96FD386DF8ABDB62D60D info_location_z_10_BEB0611A46C560C51AC03883182B74A0) (`KismetMathLibrary.MakeRotator` info_rotation_x_11_987A800F47AB53359A2C50BA5F8DEC7B info_rotation_y_12_324843F64BB1ADDB8C62A28A849F25C1 info_rotation_z_13_7CA08A5C43EFDD73901DDA8E66E6A46E)) "AlwaysSpawn" "OverrideRootScale" null (`KismetMathLibrary.MakeColor` (`KismetMathLibrary.Conv_ByteToDouble` info_red_25_A745A9FE480635E0A8A0A7A9BF7A9325) (`KismetMathLibrary.Conv_ByteToDouble` info_green_26_0F6D4FCA41095A9B1CC8EB8EB3F9DA52) (`KismetMathLibrary.Conv_ByteToDouble` info_blue_27_7D218DD644EAA95B8A1A74A422D7D039)) info_name_19_4AEED34440A6C2BDA5492B8ED0060521 null)
  (`BlueprintMapLibrary.Map_Add` (`self.Ghosts`) info_id_24_FCBBAC73426086602DE5A3BFB62D4FD0))

(fn `SyncInfo`
  (params (Info :type "/Game/Mods/BlueFireMultiplayerMod/ST_PlayerInfo Structure")))

(fn `TryRemoveGhost`
  (params (id :type Byte))
  (if (`BlueprintMapLibrary.Map_Contains` (`self.Ghosts`) id)
    (`self.RemoveGhost` id)))

(fn `UpdateGhost`
  (params (info :type "/Game/Mods/BlueFireMultiplayerMod/ST_PlayerInfo Structure"))
  (`self.K2_SetActorTransform` (`BlueprintMapLibrary.Map_Find` (`self.Ghosts`) info_id_24_FCBBAC73426086602DE5A3BFB62D4FD0) (`KismetMathLibrary.MakeTransform` (`KismetMathLibrary.MakeVector` info_location_x_2_DE92424E446ED6A7C5A5868276BA5D20 info_location_y_9_2173608E4FFA96FD386DF8ABDB62D60D info_location_z_10_BEB0611A46C560C51AC03883182B74A0) (`KismetMathLibrary.MakeRotator` info_rotation_x_11_987A800F47AB53359A2C50BA5F8DEC7B info_rotation_y_12_324843F64BB1ADDB8C62A28A849F25C1 info_rotation_z_13_7CA08A5C43EFDD73901DDA8E66E6A46E)) false true))

(fn `UpdateGhosts`
  (params (GhostInfo :type "Array of /Game/Mods/BlueFireMultiplayerMod/ST_PlayerInfo Structure") (ToRemove :type "Array of Byte"))
  (for _array_element GhostInfo
    (`self.CheckGhost` _array_element
      (:`Exists`
        (`self.UpdateGhost` _array_element))
      (:`Doesn't Exist`
        (`self.SpawnGhost` _array_element))))
  (for _array_element_2 ToRemove
    (`self.TryRemoveGhost` _array_element_2)))

(fn `UserConstructionScript`)