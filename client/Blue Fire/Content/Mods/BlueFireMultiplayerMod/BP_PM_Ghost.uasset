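; BP_PM_Ghost is an actor in the Blue Fire multiplayer mod, apparently a ghost avatar standing in for another player, with a tinted cloak and a name label.
; On BeginPlay it applies its Color to the cloak materials' ClothesColorA parameter and writes its Name to the label.
; Each Tick it billboards the label by rotating it toward the first player's camera manager.
; It contains no movement or networking logic.
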(event `self.ReceiveBeginPlay`
  (`MeshComponent.SetVectorParameterValueOnMaterials` (`self.cloak`) "ClothesColorA" (`KismetMathLibrary.Conv_LinearColorToVector` (`self.Color`)))
  (`TextRenderComponent.K2_SetText` (`self.label`) (`KismetTextLibrary.Conv_StringToText` (`self.Name`))))

(event `self.ReceiveTick`
  (params (DeltaSeconds :type "Float (single-precision)"))
  (bind _label (`self.label`))
  (`SceneComponent.K2_SetWorldRotation` _label (`KismetMathLibrary.FindLookAtRotation` (`SceneComponent.K2_GetComponentLocation` _label) (`SceneComponent.K2_GetComponentLocation` (`PlayerCameraManager.TransformComponent` (`GameplayStatics.GetPlayerCameraManager` 0)))) false false))

(fn `UserConstructionScript`)